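; bp_force is a force volume for PhysicsBallBP actors, apparently meant to steer their velocity along its Arrow, but currently it has no effect.
; Tick and ActorBeginOverlap both loop over overlapping balls with an empty loop body.
; The disconnected velocity logic clamps Arrow-local Z speed, interpolates with AdoptionSpeed and sets the ball's linear velocity.
; That logic applies InverseTransformDirection again to the result instead of transforming back to world space.
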(event `self.ReceiveTick`
  (params (DeltaSeconds :type "Float (single-precision)"))
  (for _array_element (`self.GetOverlappingActors` "/Game/RollingBP/Blueprints/PhysicsBallBP.PhysicsBallBP_C") :!label _label
    _))

(event `self.ReceiveActorBeginOverlap`
  (params (OtherActor :type "Actor Object Reference"))
  (goto _label))

(fn `UserConstructionScript`)