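; BP_ItemSpawner is an actor that spawns a random item from its ItemsToSpawn list at its own location and rotation.
; On BeginPlay it spawns one item, sets itself as owner and tracks it in CurrentItem, skipping the spawn if that item is still valid.
; The Respawn event, not called within this Blueprint, clears CurrentItem and spawns again after a configurable delay.
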(event `self.ReceiveBeginPlay`
  (`self.Attempt to spawn`))

(event `/Game/ItemSpawner/Interfaces/BPI_itemspawner.Respawn`
  (set `self.Current Item` null)
  (`KismetSystemLibrary.Delay` (`self.Delaybeforerespawn`))
  (`self.Attempt to spawn`))

(fn `Attempt to spawn`
  (`/Engine/EditorBlueprintResources/StandardMacros.IsValid` (`self.Current Item`)
    (:`Is Valid`
      (`KismetSystemLibrary.PrintString` "Item already spawned"))
    (:`Is Not Valid`
      (`self.Spawn item`))))

(fn `Spawn item`
  (bind _returnvalue (`|SpawnActorFromClass` (`|GetArrayItem` (`self.ItemsToSpawn`) (`KismetMathLibrary.RandomIntegerInRange` 0 (- (`KismetArrayLibrary.Array_Length` (`self.ItemsToSpawn`)) 1))) (`KismetMathLibrary.MakeTransform` (`self.K2_GetActorLocation`) (`self.K2_GetActorRotation`)) "AdjustIfPossibleButAlwaysSpawn" "OverrideRootScale" self null null))
  (set `self.Current Item` _returnvalue))

(fn `UserConstructionScript`)