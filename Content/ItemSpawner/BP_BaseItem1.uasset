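; BP_BaseItem1 is a power-up pickup that spins and moves in place of a static item, with only placeholder activation feedback.
; Tick adds a frame-rate-dependent yaw rotation and calls Play on the Movement timeline, whose vector track drives local offsets.
; Any actor overlap destroys the mesh, collision and particle components, then prints activation and, after a delay, deactivation messages.
; No gameplay effect is applied, and the actor itself is never destroyed.
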(event `self.ReceiveActorBeginOverlap`
  (params (OtherActor :type "Actor Object Reference"))
  ;[1 1 1] Power up
  (`ActorComponent.K2_DestroyComponent` (`self.Sphere Mesh`))
  (`ActorComponent.K2_DestroyComponent` (`self.Sphere Collison`))
  (`ActorComponent.K2_DestroyComponent` (`self.ParticleSystem`))
  (`KismetSystemLibrary.PrintString` "Powerup Activated" true true (struct :`R` 0.110038 :`G` 1.0 :`A` 1.0) 10.0)
  (`KismetSystemLibrary.Delay` 5.0)
  (`KismetSystemLibrary.PrintString` "Power up Deactivated" true true (struct :`R` 0.421875 :`G` 0.020641 :`A` 1.0) 10.0))

(event `self.ReceiveTick`
  (params (DeltaSeconds :type "Float (single-precision)"))
  ;[1 1 1] Movement of item
  (`self.K2_AddActorLocalRotation` (struct :`Yaw` 1.0))
  (bind (_direction _movememnt) (`Timeline|movement`)
    (:`Update`
      (`self.K2_AddActorLocalOffset` _movememnt))))

(fn `UserConstructionScript`)